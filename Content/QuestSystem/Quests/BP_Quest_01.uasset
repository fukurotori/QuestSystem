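; BP_Quest_01 is a quest Blueprint defining "A Long Way Home", which sends the player to reach Megaton.
; It builds a root objective collection that requires its objectives in order.
; It then fills that collection with a single reach-destination objective pointed at MegatonTrigger, constructing both objects at runtime with the quest as their outer.
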(fn `ConstructRootObjectiveCollection`
  (returns (RootObjCollection :type "/Game/QuestSystem/Objectives/BP_ObjCollections Object Reference"))
  (bind _returnvalue (`|GenericCreateObject` "/Game/QuestSystem/Objectives/BP_ObjCollections.BP_ObjCollections_C" self true "A Long Way Home"))
  (return _returnvalue))

(fn `PopulateObjectives`
  (params (RootObjCollection :type "/Game/QuestSystem/Objectives/BP_ObjCollections Object Reference"))
  (bind _returnvalue (`|GenericCreateObject` "/Game/QuestSystem/Objectives/BP_ObjReachDestination.BP_ObjReachDestination_C" self (`self.MegatonTrigger`) "Reach Megaton"))
  (`/Game/QuestSystem/Objectives/BP_ObjCollections.AddObjectives` (`local.RootObjCollection`) _returnvalue))

(fn `UserConstructionScript`
  (`parent.UserConstructionScript`))