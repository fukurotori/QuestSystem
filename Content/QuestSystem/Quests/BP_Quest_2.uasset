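; BP_Quest_2 is a quest that tasks the player with turning on a set of lamps.
; It builds a root objective collection named "Turn On Lights", then fills it with one turn-on-light objective per entry in its Lights array, each named by lamp number.
; The event graph holds only disabled default nodes, so all quest setup lives in these two construction functions.
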(fn `ConstructRootObjectiveCollection`
  (returns (RootObjCollection :type "/Game/QuestSystem/Objectives/BP_ObjCollections Object Reference"))
  (bind _returnvalue (`|GenericCreateObject` "/Game/QuestSystem/Objectives/BP_ObjCollections.BP_ObjCollections_C" self false "Turn On Lights"))
  (return _returnvalue))

(fn `PopulateObjectives`
  (params (RootObjCollection :type "/Game/QuestSystem/Objectives/BP_ObjCollections Object Reference"))
  (for (_array_element _array_index) (`self.Lights`)
    (bind _returnvalue (`|GenericCreateObject` "/Game/QuestSystem/Objectives/BP_ObjTurnOnLight.BP_ObjTurnOnLight_C" self _array_element (`|FormatText` "Turn on lamp {index}" (+ _array_index 1))))
    (`/Game/QuestSystem/Objectives/BP_ObjCollections.AddObjectives` (`local.RootObjCollection`) _returnvalue)))

(fn `UserConstructionScript`
  (`parent.UserConstructionScript`))