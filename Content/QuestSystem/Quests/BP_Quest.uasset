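; BP_Quest is a base quest Blueprint that holds a root objective collection for subclasses to define.
; On BeginPlay it constructs the root collection, stores it, then passes it to PopulateObjectives.
; ConstructRootObjectiveCollection and PopulateObjectives are override points whose base versions only print an error, and a getter exposes the stored root collection.
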(event `self.ReceiveBeginPlay`
  (bind _rootobjcollection (`self.ConstructRootObjectiveCollection`))
  (bind _output_get (set `self.RootObjectiveCollection` _rootobjcollection))
  (`self.PopulateObjectives` _output_get))

(fn `ConstructRootObjectiveCollection`
  (returns (RootObjCollection :type "/Game/QuestSystem/Objectives/BP_ObjCollections Object Reference"))
  (`KismetSystemLibrary.PrintString` "Error: CreateObjectiveCollection called for vase class!" true true (struct :`R` 1.0 :`G` 0.010197 :`B` 0.030093 :`A` 1.0))
  (return null))

(fn `GetRootObjectiveFunction`
  (returns (RootObjectiveCollection :type "/Game/QuestSystem/Objectives/BP_ObjCollections Object Reference"))
  (return (`self.RootObjectiveCollection`)))

(fn `PopulateObjectives`
  (params (RootObjCollection :type "/Game/QuestSystem/Objectives/BP_ObjCollections Object Reference"))
  (`KismetSystemLibrary.PrintString` "Error: PopulateObjectives called for vase class!" true true (struct :`R` 1.0 :`G` 0.010197 :`B` 0.030093 :`A` 1.0)))

(fn `UserConstructionScript`)